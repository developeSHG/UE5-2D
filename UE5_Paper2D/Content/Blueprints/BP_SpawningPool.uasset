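; BP_SpawningPool keeps a capped population of skeletons on the BP_TileMap that owns it.
; On BeginPlay it caches that owner and starts a self-calling spawn loop.
; Below the cap, the loop increments the count, waits a random delay and asks the tile map to spawn a BP_Skeleton; at the cap, it rechecks every tick.
; OnDespawnCreature decrements the count, freeing a slot for the next spawn.
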(event `self.ReceiveBeginPlay`
  (bind _asbp_tile_map (cast `/Game/Blueprints/BP_TileMap` (`self.GetOwner`)))
  (set `self.TileMap` _asbp_tile_map)
  (`self.UpdateRandomSpawn`))

(event `UpdateRandomSpawn`
  (if (< (`self.CreatureCount`) (`self.MaxCreatureCount`))
    (`/Engine/EditorBlueprintResources/StandardMacros.IncrementInt` (`self.CreatureCount`)
      (:`  `
        (`KismetSystemLibrary.Delay` (`KismetMathLibrary.RandomFloatInRange` 0.0 10.0))
        (`/Game/Blueprints/BP_TileMap.SpawnCreature` (`self.TileMap`) "/Game/Blueprints/Creatures/BP_Skeleton.BP_Skeleton_C")
        (`self.UpdateRandomSpawn`)))
    (else
      (`KismetSystemLibrary.DelayUntilNextTick`)
      (`self.UpdateRandomSpawn`))))

(fn `OnDespawnCreature`
  (`/Engine/EditorBlueprintResources/StandardMacros.DecrementInt` (`self.CreatureCount`)))